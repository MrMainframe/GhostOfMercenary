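; BP_BasePlayerWeapon is a base player weapon that aligns its EBBarrel component with the player's camera aim.
; UpdateBarrelLocation casts the weapon owner to BP_PlayerCharacter, caches it and reads its FollowCamera.
; It places the barrel where the camera's forward line crosses the plane facing along MuzzleLocation, then copies the camera's rotation.
; This keeps the barrel on the camera's sightline at muzzle depth.
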(event EventUpdateBarrelLocation
  (bind _muzzlelocation (Variables|Default|GetMuzzleLocation))
  (bind _asbp_player_character (Utilities|Casting|CastToBP_PlayerCharacter (Variables|Default|GetWeaponOwner)))
  (Variables|References|SetPlayerWeaponOwner _asbp_player_character)
  (Transformation|SetWorldLocation (Variables|Default|GetEBBarrel) (.Intersection (Class|KismetMathLibrary|LinePlaneIntersectionOriginNormal (Transformation|GetWorldLocation (Variables|/Game/Prototype_1/Core/Character/BP_PlayerCharacter.BP_PlayerCharacter_C|GetFollowCamera (Variables|References|GetPlayerWeaponOwner))) (+ (Transformation|GetWorldLocation (Variables|/Game/Prototype_1/Core/Character/BP_PlayerCharacter.BP_PlayerCharacter_C|GetFollowCamera (Variables|References|GetPlayerWeaponOwner))) (* (Math|Vector|GetForwardVector (Variables|/Game/Prototype_1/Core/Character/BP_PlayerCharacter.BP_PlayerCharacter_C|GetFollowCamera (Variables|References|GetPlayerWeaponOwner))) 1e+03)) (Transformation|GetWorldLocation _muzzlelocation) (Math|Vector|GetForwardVector _muzzlelocation))) false false)
  (Transformation|SetWorldRotation (Variables|Default|GetEBBarrel) (Transformation|GetWorldRotation (Variables|/Game/Prototype_1/Core/Character/BP_PlayerCharacter.BP_PlayerCharacter_C|GetFollowCamera (Variables|References|GetPlayerWeaponOwner))) false false))

(fn ConstructionScript
  (|CallParentFunction))