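; Rifle child weapon Blueprint, stored in a ToDelete folder, that supplies the cosmetic firing feedback for a parent weapon class.
; Its events play or stop the rifle fire animation on the weapon skeletal mesh and attach an emitter at the Muzzle socket for the flash.
; The rifle fire sound plays as non-spatialized 2D audio when firing ends.
; The construction script only calls the parent.
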(event EventBeginPlay
  (|CallParentFunction) ; This node is disabled and will not be called.\nDrag off pins to build functionality.
)

(event Collision|EventActorBeginOverlap
  (params (OtherActor :type Actor%20Object%20Reference))
  (|CallParentFunction OtherActor) ; This node is disabled and will not be called.\nDrag off pins to build functionality.
)

(event EventTick
  (params (DeltaSeconds :type Float%20%28single-precision%29))
  (|CallParentFunction DeltaSeconds) ; This node is disabled and will not be called.\nDrag off pins to build functionality.
)

(event EventPlayShootAnimation
  (params (IsLooping :type Boolean))
  (Components|Animation|PlayAnimation (Variables|Default|GetWeaponSkeletalMesh) "/Game/Prototype_1/Weapons/Animation/RifleAnimation/AS_FireRifle.AS_FireRifle" false))

(event EventStopAnimations
  (Audio|Components|Audio|Stop (Variables|Default|GetWeaponSkeletalMesh)))

(event EventOnFireEnd
  (Audio|PlaySound2D "/Game/Prototype_1/Weapons/Sound/Rifle/RifleFire/SC_RifleFireCue.SC_RifleFireCue" 1.0 1.0 0.0 0 0))

(event EventSpawnMuzzleFlash
  (Effects|SpawnEmitterAttached 0 (Variables|Default|GetWeaponSkeletalMesh) "Muzzle"))

(fn ConstructionScript
  (|CallParentFunction))