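; Base weapon Blueprint that handles shooting, reloading and reserve ammo for a character owner, delegating firing to an EBBarrel component.
; StartShoot and StopShoot drive the barrel, whose shot event plays montages, fire sound and AI noise.
; StartReload blocks shooting and plays the reload montage; EndReload, not called here, refills from reserve and unblocks.
; Tick calls an empty UpdateBarrelLocation while shooting, stops fire sound otherwise, and shows optional debug info.
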(event Custom|StartShoot
  ;[0.1354 0 0.002762] Start and Stop Shoot Events
  (if (not (Variables|/Script/EasyBallistics.EBBarrel|GetShootingBlocked (Variables|Default|GetEBBarrel)))
    (Variables|Shooting|SetIsShooting true)
    (Class|EBBarrel|Shoot (Variables|Default|GetEBBarrel) true)
    (if (== (Class|EBBarrel|GetAmmoCount (Variables|Default|GetEBBarrel) true) 0)
      (Audio|PlaySoundatLocation "/Game/Prototype_1/Sounds/S_AmmoEnd.S_AmmoEnd" (Transformation|GetWorldLocation (Variables|Default|GetWeaponSkeletalMesh)) "0, 0, 0" 1.0 1.0 0.0 0 0 0))))

(event Custom|StopShoot
  ;[0.1354 0 0.002762] Start and Stop Shoot Events
  (Variables|Shooting|SetIsShooting false)
  (Class|EBBarrel|Shoot (Variables|Default|GetEBBarrel) false)
  (Transformation|SetWorldTransform (Variables|Default|GetEBBarrel) (Transformation|GetWorldTransform (Variables|Default|GetMuzzleLocation)) false false)
  (Utilities|FlowControl|Delay 0.15)
  (Animation|StopAnimMontage (Variables|References|GetWeaponOwner) (Variables|Montages|GetCharacterShotMontage)))

(event Custom|OnShotFired
  ;[0.1458 0 0.003129] OnShotFired
  (Animation|Montage|PlayMontage (Variables|Default|GetWeaponSkeletalMesh) (Variables|Montages|GetWeaponShotMontage)
    (:then
      (if (Variables|Shooting|GetIsShooting)
        (Animation|Montage|PlayMontage (Variables|/Script/Engine.Character|GetMesh (Variables|References|GetWeaponOwner)) (Variables|Montages|GetCharacterShotMontage)
          (:then
            (Audio|Components|Audio|Play (Variables|Default|GetFireSound) 0.0)
            (Class|Actor|MakeNoise 5.0 0 (Transformation|GetWorldLocation (Variables|Default|GetMuzzleLocation)) 1e+03 "None")))))))

(event EventTick
  (params (DeltaSeconds :type Float%20%28single-precision%29))
  (Utilities|FlowControl|Sequence
    (:then_0
      ;[0 0.2865 0.2741] Update Barrel Location Debug
      (CallFunction|DebugDraw)
      (if (Variables|Shooting|GetIsShooting)
        (CallFunction|UpdateBarrelLocation)
        (else
          (Audio|Components|Audio|Stop (Variables|Default|GetFireSound)))))
    (:then_1
      ;[0 0.1667 0.1624] Ammo Data Print String
      (if (Variables|Debug|GetEnableDebug)
        (Development|PrintString (Utilities|String|Append (Utilities|String|BuildString(Integer) "Magazine Size" " " (Variables|Ammo|GetMagazineSize) " ") (Utilities|String|BuildString(Integer) "Max Remaining Ammo" " " (Variables|Ammo|GetMaxRemainingAmmo) " ") (Utilities|String|BuildString(Integer) "Current Remaining Ammo" " " (Variables|Ammo|GetCurrentRemainingAmmo) " ") (Utilities|String|BuildString(Integer) "Cycle Ammo Count" " " (Class|EBBarrel|GetAmmoCount (Variables|Default|GetEBBarrel) true) " ")) true true "(R=0.000000,G=0.660000,B=1.000000,A=1.000000)" 0.0)))))

(event EventBeginPlay
  ;[0 0 0] BeginPlay
  (EventDispatchers|BindEventtoShotFired (Variables|Default|GetEBBarrel) (delegate Custom|OnShotFired)))

(fn ConstructionScript)

(fn UpdateBarrelLocation)

(fn DebugDraw
  (bind _muzzlelocation (Variables|Default|GetMuzzleLocation))
  (bind _ebbarrel (Variables|Default|GetEBBarrel))
  (bind _returnvalue (Transformation|GetWorldLocation _ebbarrel))
  (bind _returnvalue_2 (Transformation|GetWorldLocation _muzzlelocation))
  (if (Variables|Debug|GetEnableDebug)
    (Rendering|Debug|DrawDebugLine _returnvalue_2 _returnvalue "(R=0.947917,G=0.088346,B=0.049371,A=1.000000)" 0.0 2.0)
    (Rendering|Debug|DrawDebugSphere _returnvalue_2 2e+01 12 "(R=1.000000,G=0.974440,B=0.045979,A=1.000000)" 0.0)
    (Rendering|Debug|DrawDebugSphere _returnvalue 2e+01 12 "(R=1.000000,G=0.974440,B=0.045979,A=1.000000)" 0.0)))

(fn StartReload
  (if (not (Variables|Reload|GetIsReloading))
    (if (> (Variables|Ammo|GetCurrentRemainingAmmo) 0)
      (CallFunction|GetRequiredAmmo)
      (if (not (== (Variables|Ammo|GetRequiredAmmoCount) 0))
        (Variables|/Script/EasyBallistics.EBBarrel|SetShootingBlocked (Variables|Default|GetEBBarrel) true)
        (Variables|Reload|SetIsReloading true)
        (bind _returnvalue (Animation|PlayAnimMontage (Variables|References|GetWeaponOwner) (Variables|Montages|GetCharacterReloadingMontage) 1.0 "None"))
        (Variables|Reload|SetReloadTime _returnvalue)
        (Audio|Components|Audio|Play (Variables|Default|GetReloadSound) 0.0)))))

(fn EndReload
  (bind _ebbarrel (Variables|Default|GetEBBarrel))
  (if (< (Variables|Ammo|GetRequiredAmmoCount) (Variables|Ammo|GetCurrentRemainingAmmo))
    (Variables|Ammo|SetCurrentRemainingAmmo (- (Variables|Ammo|GetCurrentRemainingAmmo) (Variables|Ammo|GetRequiredAmmoCount)))
    (Class|EBBarrel|SetAmmo (Variables|Default|GetEBBarrel) (+ (Class|EBBarrel|GetAmmoCount (Variables|Default|GetEBBarrel) true) (Variables|Ammo|GetRequiredAmmoCount)) true false false (Class|EBBarrel|GetAmmo (Variables|Default|GetEBBarrel) false))
    (else
      (Class|EBBarrel|SetAmmo _ebbarrel (+ (Class|EBBarrel|GetAmmoCount (Variables|Default|GetEBBarrel) true) (Variables|Ammo|GetCurrentRemainingAmmo)) true false false (Class|EBBarrel|GetAmmo _ebbarrel true))
      (Variables|Ammo|SetCurrentRemainingAmmo 0)))
  (Variables|/Script/EasyBallistics.EBBarrel|SetShootingBlocked (Variables|Default|GetEBBarrel) false)
  (Variables|Reload|SetIsReloading false))

(fn GetRequiredAmmo
  (bind _magazinesize (Variables|Ammo|GetMagazineSize))
  (Variables|Ammo|SetRequiredAmmoCount (Math|Integer|Clamp(Integer) (- _magazinesize (Class|EBBarrel|GetAmmoCount (Variables|Default|GetEBBarrel) true)) 0 _magazinesize))
  (return))

(fn GetCurrentMagazineAmmo
  (return (Class|EBBarrel|GetAmmoCount (Variables|Default|GetEBBarrel) true)))

(fn GetCurrentRemainingAmmo
  (return (Variables|Ammo|GetCurrentRemainingAmmo)))