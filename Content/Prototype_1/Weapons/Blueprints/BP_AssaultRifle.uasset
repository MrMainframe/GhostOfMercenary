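; Assault rifle weapon Blueprint that handles ammo pickups for the gun's reserve ammo.
; On PickUpAmmo, it adds a fixed magazine-sized amount to the remaining ammo, but only while the reserve is at or below a hardcoded threshold.
; The added amount is clamped to the space left under the maximum reserve.
; The construction script only calls the parent's version.
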(event Custom|PickUpAmmo
  (if (<= (Variables|Default|GetCurrentRemainingAmmo) 60)
    (Variables|Default|SetCurrentRemainingAmmo (+ (Variables|Default|GetCurrentRemainingAmmo) (Math|Integer|Clamp(Integer) 30 0 (- (Variables|Default|GetMaxRemainingAmmo) (Variables|Default|GetCurrentRemainingAmmo)))))))

(fn ConstructionScript
  (|CallParentFunction))