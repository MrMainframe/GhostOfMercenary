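; Weapon component in the AI folder that gives a character pickup, inventory, swapping, shooting, reload and melee, though built around player camera and UI.
; Pickups fill WeaponArray slots and a radial menu; equipping spawns the last picked actor's class on a mesh socket.
; Firing hitscans from player camera 0, applies damage, reports noise and loops for burst or full-auto.
; Ammo lives in the slot structs; empty clips trigger reload montages, while WeaponReload refills separately.
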(event Custom|FirePressed
  (bind _currentweapon (Variables|Weapon|GetCurrentWeapon))
  (bind _weaponconfig (Variables|/Game/Prototype_1/AI/BaseAI/System/WeaponSystem/BP_BaseWeapon.BP_BaseWeapon_C|GetWeaponConfig _currentweapon))
  (bind (_damagemin _damagemax) (Utilities|Struct|BreakS_WeaponConfig _weaponconfig))
  ;[1 0 0.2268 1 30] Fire Logic
  (if (not (Variables|Weapon|GetIsReload?))
    (Utilities|IsValid (Variables|Weapon|GetCurrentWeapon)
      (:Is%20Valid
        (if (Inventory|CheckAmmo)
          (Variables|Weapon|SetIsFire? true)
          (Variables|Weapon|SetReloadAutomatic false)
          (Weapon|SoundShooting)
          (bind (_start _end) (Utilities|LineTraceTypeWeapon)
            (:Return
              (bind _outhit (Collision|LineTraceByChannel _start _end "TraceTypeQuery1" false (Utilities|Array|MakeArray (Variables|Weapon|GetCurrentWeapon) (Variables|Weapon|GetPlayerCharacter)) "None"))
              (Game|Damage|ApplyDamage (.HitActor (Collision|BreakHitResult _outhit)) (Math|Random|RandomFloatinRange _damagemin _damagemax) 0 _currentweapon)
              (Default|WeaponMuzzleEffects (Variables|Weapon|GetCurrentWeapon) _end)
              (Camera|PlayWorldCameraShake "/Game/Prototype_1/AI/BaseAI/System/WeaponSystem/Blueprint/BP_CameraShake.BP_CameraShake_C" (Transformation|GetWorldLocation (Variables|/Script/Engine.Actor|GetRootComponent (Game|GetPlayerCameraManager 0))) 2e+02 5e+02)
              (Weapon|RemoveAmmo)
              (switch Utilities|FlowControl|Switch|SwitchonE_WeaponModeFire (Weapon|GetModeFire)
                (:NewEnumerator3
                  (bind _counter (Utilities|FlowControl|DoN 2 :!label _label)
                    (:Exit
                      (CallFunction|BurstFire 0.05)
                      (if (== _counter 2)
                        (Utilities|FlowControl|Delay 0.15)
                        (goto _label Reset)))))
                (:NewEnumerator4
                  (CallFunction|FullAutoFire)))))
          (elif (not (Variables|Weapon|GetReloadAutomatic))
            (Variables|Weapon|SetIsFire? false)
            (Variables|Weapon|SetReloadAutomatic true)
            (CallFunction|Reload)))))))

(event Custom|FireReleased
  ;[1 0 0.2268 1 30] Fire Logic
  (Variables|Weapon|SetIsFire? false))

(event Custom|PlayAnimationReload
  (bind _currentweapon (Variables|Weapon|GetCurrentWeapon))
  (bind _weaponconfig (Variables|/Game/Prototype_1/AI/BaseAI/System/WeaponSystem/BP_BaseWeapon.BP_BaseWeapon_C|GetWeaponConfig _currentweapon))
  (bind (_playeranimationreload _playeranimationmeele _playeranimationgrenade _weaponanimationreload) (Utilities|Struct|BreakS_WeaponAnimation (.animations _weaponconfig)))
  ;[0 0.3925 1 1 30] playAnimation
  (Utilities|IsValid _playeranimationreload
    (:Is%20Valid
      (Utilities|FlowControl|Sequence
        (:then_0
          (bind _returnvalue (Animation|Montage|MontagePlay (Components|SkeletalMesh|GetAnimInstance (Variables|/Script/Engine.Character|GetMesh (Variables|Weapon|GetPlayerCharacter))) _playeranimationreload 1.0 "MontageLength" 0.0 true))
          (Utilities|FlowControl|Delay _returnvalue)
          (Variables|Weapon|SetIsReload? false)
          (Variables|Weapon|SetReloadAutomatic false))
        (:then_1
          (Utilities|IsValid _weaponanimationreload
            (:Is%20Valid
              (Animation|Montage|MontagePlay (Components|SkeletalMesh|GetAnimInstance (Variables|/Game/Prototype_1/AI/BaseAI/System/WeaponSystem/BP_BaseWeapon.BP_BaseWeapon_C|GetSkeletalMesh (Variables|Weapon|GetCurrentWeapon))) _weaponanimationreload 1.0 "MontageLength" 0.0 true))))))))

(event Custom|Melee
  (bind _weaponarray (Variables|Inventory|GetWeaponArray))
  (bind _lastidweaponequip (Variables|Inventory|GetLastIDWeaponEquip))
  (bind _output (Utilities|Array|Get(acopy) _weaponarray _lastidweaponequip))
  (bind _animations (Utilities|Struct|BreakS_WeaponConfig _output))
  (bind _playeranimationmeele (Utilities|Struct|BreakS_WeaponAnimation _animations))
  ;[0 0.3925 1 1 30] playAnimation
  (if (not (Variables|Weapon|GetPlayAnimation))
    (Variables|Weapon|SetPlayAnimation true)
    (Utilities|IsValid _playeranimationmeele
      (:Is%20Valid
        (bind _returnvalue (Animation|Montage|MontagePlay (Components|SkeletalMesh|GetAnimInstance (Variables|/Script/Engine.Character|GetMesh (Variables|Weapon|GetPlayerCharacter))) _playeranimationmeele 1.0 "Duration" 0.0 true))
        (Utilities|FlowControl|Delay _returnvalue)
        (Variables|Weapon|SetPlayAnimation false)))))

(event Custom|PlayAnimationSwap
  (bind _weaponarray (Variables|Inventory|GetWeaponArray))
  (bind _lastidweaponequip (Variables|Inventory|GetLastIDWeaponEquip))
  (bind _output (Utilities|Array|Get(acopy) _weaponarray _lastidweaponequip))
  (bind _animations (Utilities|Struct|BreakS_WeaponConfig _output))
  (bind _playeranimationswap (Utilities|Struct|BreakS_WeaponAnimation _animations))
  ;[0 0.3925 1 1 30] playAnimation
  (Utilities|IsValid _playeranimationswap
    (:Is%20Valid
      (Variables|Default|SetisSwapAnimation? true)
      (bind _returnvalue (Animation|Montage|MontagePlay (Components|SkeletalMesh|GetAnimInstance (Variables|/Script/Engine.Character|GetMesh (Variables|Weapon|GetPlayerCharacter))) _playeranimationswap 1.0 "MontageLength" 0.0 true))
      (Utilities|FlowControl|Delay _returnvalue)
      (Variables|Default|SetisSwapAnimation? false))))

(event Custom|DestroyWeaponCurrent
  ;[1 0 0.4244 1 30] Destroy Weapon
  (bind _currentweapon (Variables|Weapon|GetCurrentWeapon)
    (:then
      (Actor|DestroyActor _currentweapon))
    (:else)))

(event Custom|AddWeapon
  (params (Index :type Integer) (Item :type S%20Weapon%20Config%20Structure%20%28by%20ref%29))
  ;[0 0.6406 0.04122 1 30] PickUP Weapon
  (Widget|AddWeaponMenuRadial Index)
  (Inventory|AddWeapon Index Item)
  (Weapon|SpawnWeapon Index)
  (Utilities|DestroyActor))

(event Custom|Reload
  ;[1 0 0 1 30] Reload
  (if (not (Variables|Weapon|GetIsFire?))
    (Utilities|IsValid (Variables|Weapon|GetCurrentWeapon)
      (:Is%20Valid
        (if (== (.MaxAmmo (Utilities|Struct|BreakS_WeaponConfig (Utilities|Array|Get(acopy) (Variables|Inventory|GetWeaponArray) (Variables|Inventory|GetLastIDWeaponEquip)))) 0)
          (Development|PrintString "find ammors")
          (elif (== (Utilities|Array|Get(acopy) (Variables|Inventory|GetClipSize) (Variables|Inventory|GetLastIDWeaponEquip)) (.CurrentAmmo (Utilities|Struct|BreakS_WeaponConfig (Utilities|Array|Get(acopy) (Variables|Inventory|GetWeaponArray) (Variables|Inventory|GetLastIDWeaponEquip)))))
            (Development|PrintString "Full Ammor")
            (else
              (Variables|Weapon|SetIsReload? true)
              (CallFunction|PlayAnimationReload))))))))

(event Custom|BurstFire
  (params (Duration :type Float%20%28single-precision%29))
  ;[0 0.6178 1 1 30] Mode Fire Weapon
  (Utilities|FlowControl|Delay Duration)
  (CallFunction|FirePressed))

(event Custom|Full%20Auto%20Fire
  ;[0 0.6178 1 1 30] Mode Fire Weapon
  (bind _weapon_fire_rate (Weapon|FireRateWeapon))
  (Utilities|FlowControl|Delay _weapon_fire_rate)
  (if (Variables|Weapon|GetIsFire?)
    (CallFunction|FirePressed)))

(event Custom|IsInteract
  (params (PlayerCharacter :type Character%20Object%20Reference))
  ;[0 0 0 1 30] Interact
  (if (Variables|Inventory|GetIsInteract?)
    (Utilities|FlowControl|Delay 0.2)
    (Variables|Inventory|SetIsInteract? false)
    (else
      (Variables|Inventory|SetIsInteract? true)
      (bind _hitactor (PickItem|LineTracePickUP))
      (if (Utilities|DoesObjectImplementInterface _hitactor "/Game/Prototype_1/AI/BaseAI/System/WeaponSystem/Blueprint/BP_WeaponInterface.BP_WeaponInterface_C")
        (Class|BPWeaponInterface|Interact(Message) _hitactor self PlayerCharacter)
        ;;[1 0 0.001949] DelayPickNextWeapon
        (Utilities|FlowControl|Delay 0.7)
        (Variables|Inventory|SetIsInteract? false)))))

(event Custom|WeaponModeFire
  ;[1 0 0.5307 1 30] ModeFire
  (Variables|Weapon|GetCurrentWeapon
    (:then
      (|SetModeFireLogic))
    (:else)))

(event Custom|WeaponSwap
  ;[0 0.3793 1 1 30] SwapWeapon
  (if (not (Variables|Default|GetisSwapAnimation?))
    (if (not (Variables|Weapon|GetIsFire?))
      (if (not (Variables|Weapon|GetIsSight?))
        (if (Variables|Weapon|GetIsWeaponEquip?)
          (if (Utilities|IsValidTwoWeapons)
            (Utilities|IsValid (Variables|Weapon|GetCurrentWeapon)
              (:Is%20Valid
                (bind _output_get (Variables|Inventory|SetSwapWeaponID (+ (Variables|Inventory|GetLastIDWeaponEquip) 1)))
                (if (Utilities|IsValidSwapWeapon _output_get)
                  (Variables|Inventory|SetSwapWeaponID 0))
                (Weapon|SpawnWeapon (Variables|Inventory|GetSwapWeaponID))
                (CallFunction|PlayAnimationSwap)))))))))

(event Custom|MeleeDamage
  (bind _currentweapon (Variables|Weapon|GetCurrentWeapon))
  (bind _returnvalue (Transformation|GetActorLocation _currentweapon))
  ;[0 0.3925 1 1 30] playAnimation
  (Utilities|IsValid _currentweapon
    (:Is%20Valid
      (bind _outhit (Collision|SphereTraceByChannel (+ _returnvalue 1e+01) (+ _returnvalue 2e+01) 5e+01 "TraceTypeQuery1" false 0 "None"))
      (if (!= (.HitActor (Collision|BreakHitResult _outhit)) (Variables|Weapon|GetPlayerCharacter))
        (bind _currentweapon_2 (Variables|Weapon|GetCurrentWeapon)
          (:then
            (Game|Damage|ApplyDamage (.HitActor (Collision|BreakHitResult _outhit)) 2e+01 0 _currentweapon_2))
          (:else))))))

(event Custom|PlayAnimationShooting
  (bind _currentweapon (Variables|Weapon|GetCurrentWeapon))
  (bind _weaponconfig (Variables|/Game/Prototype_1/AI/BaseAI/System/WeaponSystem/BP_BaseWeapon.BP_BaseWeapon_C|GetWeaponConfig _currentweapon))
  (bind (_playeranimationshooting _playeranimationreload _playeranimationswap _playeranimationmeele _playeranimationgrenade _weaponanimationreload _weaponanimationfire) (Utilities|Struct|BreakS_WeaponAnimation (.animations _weaponconfig)))
  ;[0 0.3925 1 1 30] playAnimation
  (Utilities|IsValid _playeranimationshooting
    (:Is%20Valid
      (Utilities|FlowControl|Sequence
        (:then_0
          (Animation|Montage|MontagePlay (Components|SkeletalMesh|GetAnimInstance (Variables|/Script/Engine.Character|GetMesh (Variables|Weapon|GetPlayerCharacter))) _playeranimationshooting 1.0 "MontageLength" 0.0 false))
        (:then_1
          (Utilities|IsValid _weaponanimationfire
            (:Is%20Valid
              (Animation|Montage|MontagePlay (Components|SkeletalMesh|GetAnimInstance (Variables|/Game/Prototype_1/AI/BaseAI/System/WeaponSystem/BP_BaseWeapon.BP_BaseWeapon_C|GetSkeletalMesh (Variables|Weapon|GetCurrentWeapon))) _weaponanimationfire 1.0 "MontageLength" 0.0 true))))))))

(event EventPickUpWeapon
  (params (Weapon :type S%20Weapon%20Config%20Structure) (PlayerCharacter :type Character%20Object%20Reference) (Actor :type BP%20Base%20Weapon%20Object%20Reference))
  ;[0 0.6406 0.04122 1 30] PickUP Weapon
  (Variables|Inventory|SetWeaponPick Weapon)
  (Variables|Weapon|SetPlayerCharacter PlayerCharacter)
  (Variables|Widget|SetActorPick Actor)
  (bind (_success_ _id) (Inventory|FindFreeStack))
  (if _success_
    (CallFunction|AddWeapon _id (Variables|Inventory|GetWeaponPick))))

(fn LineTracePickUP
  (bind _returnvalue (Game|GetPlayerCameraManager 0))
  (bind _transformcomponent (Variables|/Script/Engine.PlayerCameraManager|GetTransformComponent _returnvalue))
  (bind _returnvalue_2 (Transformation|GetWorldLocation _transformcomponent))
  (bind (_outhit _returnvalue_3) (Collision|LineTraceByChannel _returnvalue_2 (+ _returnvalue_2 (* (Math|Vector|GetForwardVector _transformcomponent) 5e+02)) "TraceTypeQuery1" false 0 "None"))
  (if _returnvalue_3
    (return (.HitActor (Collision|BreakHitResult _outhit)))))

(fn SpawnWeapon
  (params (Index :type Integer))
  (bind _output_get (Variables|Inventory|SetLastIDWeaponEquip Index))
  (Utilities|IsValid (Variables|Weapon|GetCurrentWeapon)
    (:Is%20Valid
      (Actor|DestroyActor (Variables|Weapon|GetCurrentWeapon)))
    (:Is%20Not%20Valid
      _))
  (bind _returnvalue (Game|SpawnActorfromClass :Class (Utilities|GetClass (Variables|Widget|GetActorPick)) :SpawnTransform (Transformation|GetSocketTransform (Variables|/Script/Engine.Character|GetMesh (Variables|Weapon|GetPlayerCharacter)) (.SocketWeapon (Utilities|Struct|BreakS_WeaponConfig (Utilities|Array|Get(acopy) (Variables|Inventory|GetWeaponArray) _output_get))) "RTS_World") :CollisionHandlingOverride "Undefined" :Instigator 0))
  (Development|PrintString (Utilities|GetDisplayName _returnvalue))
  (Variables|Weapon|SetCurrentWeapon _returnvalue)
  (Variables|Weapon|SetSwitch%20Firing%20Modes (.WeaponModeFire (Utilities|Struct|BreakS_WeaponConfig (Utilities|Array|Get(acopy) (Variables|Inventory|GetWeaponArray) _output_get))))
  (Variables|Inventory|SetWeaponID (.IDWeapon (Utilities|Struct|BreakS_WeaponConfig (Utilities|Array|Get(acopy) (Variables|Inventory|GetWeaponArray) _output_get))))
  (Transformation|AttachComponentToComponent _returnvalue (Variables|/Script/Engine.Character|GetMesh (Variables|Weapon|GetPlayerCharacter)) (.SocketWeapon (Utilities|Struct|BreakS_WeaponConfig (Utilities|Array|Get(acopy) (Variables|Inventory|GetWeaponArray) _output_get))) "SnapToTarget" "SnapToTarget" "SnapToTarget" true)
  (Default|SetWeaponState _returnvalue "NewEnumerator1")
  (Variables|Weapon|SetIsWeaponEquip? true)
  (Weapon|SwitchModeFire "NewEnumerator0")
  (return))

(fn FindFreeStack
  (bind (_array_element _array_index) (Utilities|Array|ForEachLoopwithBreak (Variables|Inventory|GetWeaponArray) :!label _label)
    (:LoopBody
      (if (Utilities|Enum|Equal(Enum) (.name (Utilities|Struct|BreakS_WeaponConfig _array_element)) "")
        (LocalVariables|SetLocal_Found true)
        (LocalVariables|SetLocal_ID _array_index)
        (goto _label Break)))
    (:Completed
      (return (LocalVariables|GetLocal_Found) (LocalVariables|GetLocal_ID)))))

(fn AddWeapon
  (params (Index :type Integer) (Item :type S%20Weapon%20Config%20Structure%20%28by%20ref%29))
  (bind (_idweapon _damagemin _damagemax _currentammo _maxammo) (Utilities|Struct|BreakS_WeaponConfig Item))
  (Utilities|Array|SetArrayElem (Variables|Inventory|GetWeaponArray) Index Item)
  (Utilities|Array|SetArrayElem (Variables|Inventory|GetClipSize) Index _currentammo)
  (Utilities|Array|SetArrayElem (Variables|Inventory|GetMaxAmmo) Index _maxammo))

(fn SpawnWidgets
  (params (PlayerController :type Player%20Controller%20Object%20Reference) (PlayerCharacter :type Character%20Object%20Reference))
  (Variables|Weapon|SetPlayerController PlayerController)
  (Variables|Weapon|SetPlayerCharacter PlayerCharacter)
  (bind _returnvalue (UserInterface|CreateWidget "/Game/Prototype_1/AI/BaseAI/System/WeaponSystem/Widget/WB_HUDWeapon.WB_HUDWeapon_C"))
  (UserInterface|Viewport|AddtoViewport _returnvalue 0)
  (bind _returnvalue_2 (UserInterface|CreateWidget "/Game/Prototype_1/AI/BaseAI/System/MenuRadial/Blueprint/WB_RadialMenu.WB_RadialMenu_C" (Variables|Weapon|GetPlayerController) self))
  (bind _output_get (Variables|Widget|SetRadialMenu _returnvalue_2))
  (UserInterface|Viewport|AddtoViewport _output_get 0)
  (Widget|SetVisibility _returnvalue_2 "Hidden"))

(fn Open/CloseMenuWeapons
  (bind _playercharacter (Variables|Weapon|GetPlayerCharacter))
  (bind _charactermovement (Variables|/Script/Engine.Character|GetCharacterMovement _playercharacter))
  (if (Variables|Widget|GetIsShowMenuWeapons?)
    (Widget|CloseMenuWeapons)
    (else
      (Widget|SetVisibility (Variables|Widget|GetRadialMenu) "Visible")
      (Variables|/Script/Engine.PlayerController|SetbShowMouseCursor (Variables|Weapon|GetPlayerController) true)
      (Variables|Widget|SetIsShowMenuWeapons? true)
      (Pawn|Components|CharacterMovement|DisableMovement _charactermovement)
      (Components|Movement|StopMovementImmediately _charactermovement)
      (Input|SetInputModeGameandUI (Variables|Weapon|GetPlayerController) (Variables|Widget|GetRadialMenu) "DoNotLock" true))))

(fn CloseMenuWeapons
  (if (Variables|Widget|GetIsShowMenuWeapons?)
    (Widget|SetVisibility (Variables|Widget|GetRadialMenu) "Hidden")
    (Variables|/Script/Engine.PlayerController|SetbShowMouseCursor (Variables|Weapon|GetPlayerController) false)
    (Pawn|Components|CharacterMovement|SetMovementMode (Variables|/Script/Engine.Character|GetCharacterMovement (Variables|Weapon|GetPlayerCharacter)) "MOVE_Walking" 0)
    (Input|SetInputModeGameOnly (Variables|Weapon|GetPlayerController))
    (Variables|Widget|SetIsShowMenuWeapons? false)))

(fn AddWeaponMenuRadial
  (params (ID :type Integer))
  (bind _radialmenu (Variables|Widget|GetRadialMenu))
  (bind _wb_radialmenubase (Variables|/Game/Prototype_1/AI/BaseAI/System/MenuRadial/Blueprint/WB_RadialMenu.WB_RadialMenu_C|GetWB_RadialMenuBase _radialmenu))
  (Utilities|IsValid _radialmenu
    (:Is%20Valid
      (Utilities|IsValid _wb_radialmenubase
        (:Is%20Valid
          (Default|UpdateIcon _wb_radialmenubase ID (.Icon (Utilities|Struct|BreakS_WeaponConfig (Variables|Inventory|GetWeaponPick)))))))))

(fn CheckWeaponFound
  (params (ID :type Integer))
  (return (not (Utilities|Enum|Equal(Enum) (.name (Utilities|Struct|BreakS_WeaponConfig (Utilities|Array|Get(acopy) (Variables|Inventory|GetWeaponArray) ID))) ""))))

(fn CheckAmmo
  (return (> (.CurrentAmmo (Utilities|Struct|BreakS_WeaponConfig (Utilities|Array|Get(acopy) (Variables|Inventory|GetWeaponArray) (Variables|Inventory|GetLastIDWeaponEquip)))) 0)))

(fn RemoveAmmo
  (bind _weaponarray (Variables|Inventory|GetWeaponArray))
  (bind _lastidweaponequip (Variables|Inventory|GetLastIDWeaponEquip))
  (bind _output (Utilities|Array|Get(acopy) _weaponarray _lastidweaponequip))
  (bind _structout (Utilities|Struct|SetmembersinS_WeaponConfig _output (- (.CurrentAmmo (Utilities|Struct|BreakS_WeaponConfig _output)) 1)))
  (Utilities|Array|SetArrayElem (Variables|Inventory|GetWeaponArray) (Variables|Inventory|GetLastIDWeaponEquip) _structout))

(fn SoundShooting
  (bind _currentweapon (Variables|Weapon|GetCurrentWeapon))
  (bind _currentweapon_2 (Variables|Weapon|GetCurrentWeapon))
  (bind _weaponconfig (Variables|/Game/Prototype_1/AI/BaseAI/System/WeaponSystem/BP_BaseWeapon.BP_BaseWeapon_C|GetWeaponConfig _currentweapon))
  (Class|AISenseHearing|ReportNoiseEvent (Transformation|GetActorLocation _currentweapon_2) 2e+03 _currentweapon_2 0.0 "None")
  (Utilities|IsValid (.soundshooting _weaponconfig)
    (:Is%20Valid
      (Audio|PlaySoundatLocation (.soundshooting _weaponconfig) (Transformation|GetWorldLocation (Variables|/Game/Prototype_1/AI/BaseAI/System/WeaponSystem/BP_BaseWeapon.BP_BaseWeapon_C|GetMuzzle _currentweapon)) "0, 0, 0" 1.0 1.0 0.0 0 0 0)
      (return))
    (:Is%20Not%20Valid
      (return))))

(fn GetModeFire
  (return (.WeaponModeFire (Utilities|Struct|BreakS_WeaponConfig (Utilities|Array|Get(acopy) (Variables|Inventory|GetWeaponArray) (Variables|Inventory|GetLastIDWeaponEquip))))))

(fn FireRateWeapon
  (return (.firerate (Variables|/Game/Prototype_1/AI/BaseAI/System/WeaponSystem/BP_BaseWeapon.BP_BaseWeapon_C|GetWeaponConfig (Variables|Weapon|GetCurrentWeapon)))))

(fn SwitchModeFire
  (params (WeaponModeFire :type E_WeaponModeFire%20Enum :default "NewEnumerator2"))
  (bind _structout (Utilities|Struct|SetmembersinS_WeaponConfig (Utilities|Array|Get(acopy) (Variables|Inventory|GetWeaponArray) (Variables|Inventory|GetLastIDWeaponEquip)) WeaponModeFire))
  (Utilities|Array|SetArrayElem (Variables|Inventory|GetWeaponArray) (Variables|Inventory|GetLastIDWeaponEquip) _structout)
  (return))

(fn GetCurrentAmmo
  (return (.CurrentAmmo (Utilities|Struct|BreakS_WeaponConfig (Utilities|Array|Get(acopy) (Variables|Inventory|GetWeaponArray) (Variables|Inventory|GetLastIDWeaponEquip))))))

(fn WeaponReload
  (bind _weaponarray (Variables|Inventory|GetWeaponArray))
  (bind _lastidweaponequip (Variables|Inventory|GetLastIDWeaponEquip))
  (bind _lastidweaponequip_2 (Variables|Inventory|GetLastIDWeaponEquip))
  (bind _weaponarray_2 (Variables|Inventory|GetWeaponArray))
  (bind _lastidweaponequip_3 (Variables|Inventory|GetLastIDWeaponEquip))
  (bind _weaponarray_3 (Variables|Inventory|GetWeaponArray))
  (bind _output (Utilities|Array|Get(acopy) _weaponarray _lastidweaponequip_2))
  (bind _output_2 (Utilities|Array|Get(acopy) _weaponarray_2 _lastidweaponequip_3))
  (bind _output_3 (Utilities|Array|Get(acopy) _weaponarray_3 _lastidweaponequip))
  (bind (_animationblueprint _idweapon _damagemin _damagemax _currentammo _maxammo) (Utilities|Struct|BreakS_WeaponConfig _output))
  (bind _maxammo_2 (Utilities|Struct|BreakS_WeaponConfig _output_3))
  (bind (_animationblueprint_2 _idweapon_2 _damagemin_2 _damagemax_2 _currentammo_2 _maxammo_3) (Utilities|Struct|BreakS_WeaponConfig _output_2))
  (if (> _maxammo 0)
    (Variables|Weapon|SetNeedAmmo (- (Utilities|Array|Get(acopy) (Variables|Inventory|GetClipSize) (Variables|Inventory|GetLastIDWeaponEquip)) _currentammo))
    (if (<= _maxammo_2 (Variables|Weapon|GetNeedAmmo))
      (bind _structout (Utilities|Struct|SetmembersinS_WeaponConfig (Utilities|Array|Get(acopy) (Variables|Inventory|GetWeaponArray) (Variables|Inventory|GetLastIDWeaponEquip)) (+ _currentammo_2 _maxammo_3)))
      (Utilities|Array|SetArrayElem (Variables|Inventory|GetWeaponArray) (Variables|Inventory|GetLastIDWeaponEquip) _structout)
      (else
        (bind _structout_2 (Utilities|Struct|SetmembersinS_WeaponConfig (Utilities|Array|Get(acopy) (Variables|Inventory|GetWeaponArray) (Variables|Inventory|GetLastIDWeaponEquip)) (Utilities|Array|Get(acopy) (Variables|Inventory|GetClipSize) (Variables|Inventory|GetLastIDWeaponEquip)) (- _maxammo_2 (Variables|Weapon|GetNeedAmmo))))
        (Utilities|Array|SetArrayElem (Variables|Inventory|GetWeaponArray) (Variables|Inventory|GetLastIDWeaponEquip) _structout_2)))))

(fn GetMaxAmmo
  (return (.MaxAmmo (Utilities|Struct|BreakS_WeaponConfig (Utilities|Array|Get(acopy) (Variables|Inventory|GetWeaponArray) (Variables|Inventory|GetLastIDWeaponEquip))))))

(fn AddAmmo
  (if (== (.MaxAmmo (Utilities|Struct|BreakS_WeaponConfig (Utilities|Array|Get(acopy) (Variables|Inventory|GetWeaponArray) (Variables|Inventory|GetLastIDWeaponEquip)))) (Utilities|Array|Get(acopy) (Variables|Inventory|GetMaxAmmo) (Variables|Inventory|GetLastIDWeaponEquip)))
    (return false)
    (else
      (bind _structout (Utilities|Struct|SetmembersinS_WeaponConfig (Utilities|Array|Get(acopy) (Variables|Inventory|GetWeaponArray) (Variables|Inventory|GetLastIDWeaponEquip)) (Utilities|Array|Get(acopy) (Variables|Inventory|GetMaxAmmo) (Variables|Inventory|GetLastIDWeaponEquip))))
      (Utilities|Array|SetArrayElem (Variables|Inventory|GetWeaponArray) (Variables|Inventory|GetLastIDWeaponEquip) _structout)
      (return true))))