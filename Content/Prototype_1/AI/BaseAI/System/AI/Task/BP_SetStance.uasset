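; Behavior Tree task that sets the stance of the AI-controlled pawn.
; On execute it switches on its Stance variable and sends that value to the pawn through a SetStance message call.
; Crouch and Standing always send it, while Random sends the Random value itself on a coin flip and otherwise leaves the pawn untouched.
; All handled paths finish immediately with success.
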(event EventReceiveExecuteAI
  (params (OwnerController :type AI%20Controller%20Object%20Reference) (ControlledPawn :type Pawn%20Object%20Reference))
  (switch Utilities|FlowControl|Switch|SwitchonE_SetStance (Variables|Default|GetStance)
    (:NewEnumerator0
      (Class|BPAIinterface|SetStance(Message) ControlledPawn (Variables|Default|GetStance) :!label _label)
      (AI|BehaviorTree|FinishExecute true))
    (:NewEnumerator1
      (goto _label))
    (:NewEnumerator2
      (if (Math|Random|RandomBool)
        (Class|BPAIinterface|SetStance(Message) ControlledPawn (Variables|Default|GetStance))
        (AI|BehaviorTree|FinishExecute true)
        (else
          (AI|BehaviorTree|FinishExecute true))))))