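; Behavior tree task that sends the controlled pawn a fire message using its Fire variable.
; If the blackboard Target reports dead, it stops firing and finishes.
; Otherwise it finishes at once, while a retriggerable random delay of a few seconds later sends the stop message, so firing can outlast the task.
; Aborting also stops firing.
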(event EventReceiveExecuteAI
  (params (OwnerController :type AI%20Controller%20Object%20Reference) (ControlledPawn :type Pawn%20Object%20Reference))
  (Class|BPAIinterface|Fire(Message) ControlledPawn (Variables|Default|GetFire?))
  (bind _dead_ (Class|BPAIShooterInterface|Dead?(Message) (AI|BehaviorTree|GetBlackboardValueasActor (Variables|Default|GetTarget))))
  (if _dead_
    (Class|BPAIinterface|Fire(Message) ControlledPawn false)
    (AI|BehaviorTree|FinishExecute true)
    (else
      (Utilities|FlowControl|Sequence
        (:then_0
          (Utilities|FlowControl|RetriggerableDelay (Math|Random|RandomFloatinRange 2.0 4.0))
          (Class|BPAIinterface|Fire(Message) ControlledPawn false))
        (:then_1
          (AI|BehaviorTree|FinishExecute true))))))

(event EventReceiveAbortAI
  (params (OwnerController :type AI%20Controller%20Object%20Reference) (ControlledPawn :type Pawn%20Object%20Reference))
  (|CallParentFunction OwnerController ControlledPawn)
  (Class|BPAIinterface|Fire(Message) ControlledPawn false)
  (Class|BTTaskBlueprintBase|FinishAbort))