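; Base enemy weapon Blueprint for the prototype's test AI, built on a parent weapon class.
; On UpdateBarrelLocation, it casts the weapon owner to BP_AITerrorEnemy and, if that enemy's controller has a valid target, rotates the EBBarrel component in world space to face it.
; A rifle fire loop sound node is present but unconnected, and the construction script only calls the parent.
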(event EventUpdateBarrelLocation
  (bind _asbp_aiterror_enemy (Utilities|Casting|CastToBP_AITerrorEnemy (Variables|Default|GetWeaponOwner)))
  (Utilities|IsValid (Variables|/Game/Prototype_1/AI/TestAI/AIC_BaseEnemy.AIC_BaseEnemy_C|GetTargetEnemy (Variables|/Game/Prototype_1/AI/TestAI/BP_AITerrorEnemy.BP_AITerrorEnemy_C|GetControllerRef _asbp_aiterror_enemy))
    (:Is%20Valid
      (Transformation|SetWorldRotation (Variables|Default|GetEBBarrel) (Math|Rotator|FindLookatRotation (Transformation|GetWorldLocation (Variables|Default|GetEBBarrel)) (Transformation|GetActorLocation (Variables|/Game/Prototype_1/AI/TestAI/AIC_BaseEnemy.AIC_BaseEnemy_C|GetTargetEnemy (Variables|/Game/Prototype_1/AI/TestAI/BP_AITerrorEnemy.BP_AITerrorEnemy_C|GetControllerRef _asbp_aiterror_enemy)))) false false))))

(fn ConstructionScript
  (|CallParentFunction))