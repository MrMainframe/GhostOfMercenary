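; BP_EQSTestEnemy is a test enemy character for EQS AI, with a child-actor weapon and an overhead health bar.
; On BeginPlay it caches its AIC_EQSTestEnemy controller, assigns itself as the weapon's owner and links itself to the health bar widget.
; While the controller has a valid target, Tick turns the health bar toward the player camera.
; On death it calls the parent logic, stops shooting and collapses the bar.
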(event EventBeginPlay
  (Utilities|FlowControl|Sequence
    (:then_0
      ;[1 1 1] Controller Ref
      (bind _asaic_eqstest_enemy (Utilities|Casting|CastToAIC_EQSTestEnemy (Pawn|GetController)))
      (Variables|Default|SetControllerRef _asaic_eqstest_enemy))
    (:then_1
      ;[1 1 1] Set AI Weapon Owner
      (bind _asbp_weapon_base (Utilities|Casting|CastToBP_WeaponBase (Variables|/Script/Engine.ChildActorComponent|GetChildActor (Variables|Default|GetWeaponActor))))
      (bind _output_get (Variables|Default|SetCurrentWeapon _asbp_weapon_base))
      (Variables|/Game/Prototype_1/Weapons/Blueprints/BP_WeaponBase.BP_WeaponBase_C|SetWeaponOwner _output_get self))
    (:then_2
      ;[1 1 1] Health Bar
      (bind _aswbp_health_bar (Utilities|Casting|CastToWBP_HealthBar (UserInterface|GetUserWidgetObject (Variables|Default|GetHealthBarComponent))))
      (Variables|Default|SetHPBarRef _aswbp_health_bar)
      (Variables|/Game/Prototype_1/Widgets/Bars/WBP_HealthBar.WBP_HealthBar_C|SetOwnerCharacter _aswbp_health_bar self))))

(event EventOnDeath
  ;[1 1 1] Event On Death
  (|CallParentFunction)
  (Default|StopShoot (Variables|Default|GetCurrentWeapon))
  (Widget|SetVisibility (Variables|Default|GetHPBarRef) "Collapsed"))

(event EventTick
  (params (DeltaSeconds :type Float%20%28single-precision%29))
  (bind _healthbarcomponent (Variables|Default|GetHealthBarComponent))
  ;[1 1 1] Rotation AI Health Bar For Player
  (Utilities|IsValid (Variables|/Game/Prototype_1/AI/TestAI/EQS/EQS_Test/AIC_EQSTestEnemy.AIC_EQSTestEnemy_C|GetTargetEnemy (Variables|Default|GetControllerRef))
    (:Is%20Valid
      (Transformation|SetWorldRotation _healthbarcomponent (Math|Rotator|FindLookatRotation (Transformation|GetWorldLocation _healthbarcomponent) (Camera|GetCameraLocation (Game|GetPlayerCameraManager 0))) false false))))

(fn ConstructionScript)