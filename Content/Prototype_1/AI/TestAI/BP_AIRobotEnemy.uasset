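; Robot enemy Blueprint for the prototype's test AI, with almost no live logic of its own.
; BeginPlay only casts its controller to AIC_BaseEnemy; the death event, Tick and construction script are empty.
; Disconnected leftover nodes cover death cleanup, health bar owner setup, turning the bar toward the player camera and assigning the weapon owner, none of which runs.
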(event EventBeginPlay
  (Utilities|FlowControl|Sequence
    (:then_0
      ;[1 1 1] Controller Ref
      (Utilities|Casting|CastToAIC_BaseEnemy (Pawn|GetController)))
    (:then_1)
    (:then_2)))

(event EventOnDeath
  ;[1 1 1] Event On Death
)

(event EventTick
  (params (DeltaSeconds :type Float%20%28single-precision%29)))

(fn ConstructionScript)