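; Base character Blueprint that provides health, damage handling and death, apparently as a parent for other characters.
; AnyDamage subtracts from current health within a clamped range and triggers OnDeath when it reaches zero.
; OnDeath sets the dead flag, then, if the mesh is valid, starts the death montage and calls the OnDead and OnPostDead dispatchers.
; GetHP returns health as a normalized fraction of maximum.
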(event Custom|OnDeath
  (bind _mesh (Variables|Character|GetMesh))
  ;[0 0 0] Event OnDeath
  (Variables|DeathSystem|SetIsDead true)
  (Utilities|IsValid _mesh
    (:Is%20Valid
      (Animation|Montage|PlayMontage _mesh (Variables|DeathSystem|GetDeathMontage)
        (:then
          (Default|CallOnDead)
          (Default|CallOnPostDead))))))

(event Game|Damage|EventAnyDamage
  (params (Damage :type Float%20%28single-precision%29) (DamageType :type Damage%20Type%20Object%20Reference) (InstigatedBy :type Controller%20Object%20Reference) (DamageCauser :type Actor%20Object%20Reference))
  ;[0 0 0] Event Damage
  (if (> (Variables|HealthSystem|GetCurrentHealth) 0.0)
    (bind _output_get (Variables|HealthSystem|SetCurrentHealth (Math|Float|Clamp(Float) (- (Variables|HealthSystem|GetCurrentHealth) Damage) 0.0 (Variables|HealthSystem|GetMaxHealth))))
    (if (<= _output_get 0.0)
      (CallFunction|OnDeath))))

(fn ConstructionScript)

(fn GetHP
  (return (Math|Float|Clamp(Float) (/ (Variables|HealthSystem|GetCurrentHealth) (Variables|HealthSystem|GetMaxHealth)))))