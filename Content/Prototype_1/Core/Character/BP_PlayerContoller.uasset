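; Player controller for the Prototype_1 game that toggles the pause menu on the GamePause input action.
; On press it flips an IsGamePaused flag, then either creates WBP_PauseMenu, shows the cursor and switches to game-and-UI input focused on the menu, or removes the menu and restores game-only input.
; The game's paused state is set to match each toggle.
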(event Input|ActionEvents|InputActionGamePause
  (params (Key :type Key%20Structure :default "None"))
  (:Pressed
    (if (Variables|Default|GetIsGamePaused)
      (Variables|Default|SetIsGamePaused false)
      (Widget|RemovefromParent (stale _returnvalue))
      (Variables|Default|SetbShowMouseCursor false)
      (Input|SetInputModeGameOnly self)
      (Game|SetGamePaused false)
      (else
        (Variables|Default|SetIsGamePaused true)
        (bind _returnvalue (UserInterface|CreateWidget "/Game/Prototype_1/Widgets/PauseMenu/WBP_PauseMenu.WBP_PauseMenu_C"))
        (UserInterface|Viewport|AddtoViewport _returnvalue 0)
        (Variables|Default|SetbShowMouseCursor true)
        (Input|SetInputModeGameandUI self _returnvalue "DoNotLock" true)
        (Game|SetGamePaused true)))))

(fn ConstructionScript)