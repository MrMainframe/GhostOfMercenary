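; Land turret actor that tracks and shoots at the player until its HP runs out, then explodes.
; Each tick while the player lives, a line trace from the right muzzle gates interpolated, pitch-clamped rotation of gun and swivel.
; Fire rate and a dot-product facing check trigger Firing, which checks sight and range, then shoots both EBBarrels staggered by a delay.
; Lost sight calls the same Fire event to switch the barrels off.
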(event Custom|Fire
  ;[0 0 0] Firing
  (|Firing))

(event Game|Damage|EventAnyDamage
  (params (Damage :type Float%20%28single-precision%29) (DamageType :type Damage%20Type%20Object%20Reference) (InstigatedBy :type Controller%20Object%20Reference) (DamageCauser :type Actor%20Object%20Reference))
  (bind _returnvalue (Transformation|GetActorLocation))
  ;[0 0 0] Turret Destroy
  (if (> (Variables|Constant|GetTurretHP) 0.0)
    (bind _output_get (Variables|Constant|SetTurretHP (- (Variables|Constant|GetTurretHP) Damage)))
    (if (<= _output_get 0.0)
      (Actor|DestroyActor)
      (Audio|PlaySoundatLocation "/Game/Prototype_1/Sounds/Explosion/Explosion_Cue.Explosion_Cue" _returnvalue "0, 0, 0" 1.0 1.0 0.0 0 0 0)
      (Effects|SpawnEmitteratLocation "/Game/Prototype_1/Particles/Explosion/P_Explosion_Barrel.P_Explosion_Barrel" _returnvalue))))

(event EventBeginPlay
  ;[0 0 0] PlayerRef
  (bind _asbp_player_character (Utilities|Casting|CastToBP_PlayerCharacter (Game|GetPlayerCharacter 0)))
  (Variables|Reference|SetPlayerRef _asbp_player_character))

(event EventTick
  (params (DeltaSeconds :type Float%20%28single-precision%29))
  (bind _playerref (Variables|Reference|GetPlayerRef))
  ;[0 0 0] Rotation and firing
  (if (not (Variables|/Game/Prototype_1/Core/Character/BP_BaseCharacter.BP_BaseCharacter_C|GetIsDead _playerref))
    (CallFunction|Rotation _playerref)
    (CallFunction|UpdateFire)))

(fn ConstructionScript)

(fn Rotation
  (params (PlayerRef :type Actor%20Object%20Reference))
  ;[0 0 0] Set Locations of Turret and Player
  (bind _output_get (Variables|Location|SetPlayerLocation (Transformation|GetActorLocation PlayerRef)))
  (bind _output_get_2 (Variables|Location|SetTurretLocation (Transformation|GetWorldLocation (Variables|Default|GetStand))))
  ;[0 0 0] Set axis of rotation
  (Variables|Constant|SetXRotation (.roll (Math|Rotator|FindLookatRotation _output_get_2 _output_get)))
  (Variables|Constant|SetYRotation (.pitch (Math|Rotator|FindLookatRotation _output_get_2 _output_get)))
  (Variables|Constant|SetZRotation (.yaw (Math|Rotator|FindLookatRotation _output_get_2 _output_get)))
  ;[0 0 0] Chechking player in vision for rotation
  (bind _outhit (Collision|LineTraceForObjects (Transformation|GetWorldLocation (Variables|Default|GetRightMuzzleLocation)) (Variables|Location|GetPlayerLocation) (Utilities|Array|MakeArray "ObjectTypeQuery3" "ObjectTypeQuery1" "ObjectTypeQuery2" "ObjectTypeQuery4") false 0 "None"))
  (Variables|Booleans|SetbPlayerInVision? (== (.hitactor _outhit) (Variables|Reference|GetPlayerRef)))
  (if (Variables|Booleans|GetbPlayerInVision?)
    ;[0 0 0] Set Turret Rotation
    (Transformation|SetWorldRotation (Variables|Default|GetGun) (Math|Rotator|MakeRotator (.pitch (Math|Interpolation|RInterpTo (Transformation|GetWorldRotation (Variables|Default|GetGun)) (Math|Rotator|MakeRotator 0.0 (Math|Float|ClampAngle (* (Variables|Constant|GetYRotation) -1.0) -9e+01 3e+01) (- (Variables|Constant|GetZRotation) 9e+01)) (Utilities|Time|GetWorldDeltaSeconds) (Variables|Constant|GetRotationSpeed))) 0.0 (.yaw (Math|Interpolation|RInterpTo (Transformation|GetWorldRotation (Variables|Default|GetGun)) (Math|Rotator|MakeRotator 0.0 (Math|Float|ClampAngle (* (Variables|Constant|GetYRotation) -1.0) -9e+01 3e+01) (- (Variables|Constant|GetZRotation) 9e+01)) (Utilities|Time|GetWorldDeltaSeconds) (Variables|Constant|GetRotationSpeed)))) false false)
    (Transformation|SetWorldRotation (Variables|Default|GetSwivel) (Math|Rotator|MakeRotator (.pitch (Math|Interpolation|RInterpTo (Transformation|GetWorldRotation (Variables|Default|GetGun)) (Math|Rotator|MakeRotator 0.0 (Math|Float|ClampAngle (* (Variables|Constant|GetYRotation) -1.0) -9e+01 3e+01) (- (Variables|Constant|GetZRotation) 9e+01)) (Utilities|Time|GetWorldDeltaSeconds) (Variables|Constant|GetRotationSpeed))) 0.0 (.yaw (Math|Interpolation|RInterpTo (Transformation|GetWorldRotation (Variables|Default|GetGun)) (Math|Rotator|MakeRotator 0.0 (Math|Float|ClampAngle (* (Variables|Constant|GetYRotation) -1.0) -9e+01 3e+01) (- (Variables|Constant|GetZRotation) 9e+01)) (Utilities|Time|GetWorldDeltaSeconds) (Variables|Constant|GetRotationSpeed)))) false false)
    (return)
    (else
      (CallFunction|Fire) ; Stop Fire
    )))

(fn FireandDistance)

(fn UpdateFire
  (if (> (- (Utilities|Time|GetGameTimeinSeconds) (Variables|Constant|GetTimeOfLastFire)) (Variables|Constant|GetRateOfFire))
    (if (> (+ (Math|Vector|DotProduct (Math|Vector|GetUnitDirection(Vector) (Transformation|GetWorldLocation (Variables|Default|GetGun)) (Transformation|GetActorLocation (Variables|Reference|GetPlayerRef))) (Math|Vector|GetForwardVector (Variables|Default|GetGun))) 1.0) 0.99)
      (CallFunction|Fire))))