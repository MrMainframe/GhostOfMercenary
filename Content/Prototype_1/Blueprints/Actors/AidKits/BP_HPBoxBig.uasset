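; BP_HPBoxBig is a large health box pickup that refills the player's health.
; Any overlap with ActivationZone fetches the first BP_PlayerCharacter without checking the overlapping actor, calling HPBigBoxRefill and playing a sound if health is below 100.
; Its Widget spins on Tick and bobs through two timelines that restart each other.
; The box has no destroy or cooldown logic.
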(event OnComponentBeginOverlap(ActivationZone)
  (params (OverlappedComponent :type Primitive%20Component%20Object%20Reference) (OtherActor :type Actor%20Object%20Reference) (OtherComp :type Primitive%20Component%20Object%20Reference) (OtherBodyIndex :type Integer) (bFromSweep :type Boolean) (SweepResult :type Hit%20Result%20Structure%20%28by%20ref%29))
  (bind _outactors (Actor|GetAllActorsOfClass "/Game/Prototype_1/Core/Character/BP_PlayerCharacter.BP_PlayerCharacter_C"))
  (bind _asbp_player_character (Utilities|Casting|CastToBP_PlayerCharacter (Utilities|Array|Get(acopy) _outactors)))
  (if (< (Variables|/Game/Prototype_1/Core/Character/BP_BaseCharacter.BP_BaseCharacter_C|GetCurrentHealth _asbp_player_character) 1e+02)
    (Default|HPBigBoxRefill _asbp_player_character)
    (Audio|SpawnSoundatLocation "/Game/Prototype_1/Sounds/S_HPRefill.S_HPRefill" (Transformation|GetWorldLocation (Variables|Default|GetSM_HPBox_Big)) "0, 0, 0" 1.0 1.0 0.0 0 0)))

(event EventBeginPlay
  (bind _uplocation (Timeline|WidgetUP Play)
    (:Update
      (Transformation|AddRelativeLocation (Variables|Default|GetWidget) _uplocation false false))
    (:Finished
      (bind _downlocation (Timeline|WidgetDown PlayFromStart)
        (:Update
          (Transformation|AddRelativeLocation (Variables|Default|GetWidget) _downlocation false false))
        (:Finished
          (Timeline|WidgetUP PlayFromStart))))))

(event EventTick
  (params (DeltaSeconds :type Float%20%28single-precision%29))
  (Transformation|AddRelativeRotation (Variables|Default|GetWidget) (* (Math|Rotator|MakeRotator 0.0 0.0 1e+02) DeltaSeconds) false false))

(fn ConstructionScript)