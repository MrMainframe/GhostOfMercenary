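; Pistol ammo pickup that refills the pistol when the player overlaps its activation zone.
; On overlap it finds the first BP_Pistol in the level and, if its remaining ammo is below a fixed cap, calls PickUpAmmo, plays a refill sound and destroys itself.
; BeginPlay caches the player and starts two alternating timelines that endlessly bob three widget components up and down, while Tick spins the first one.
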(event OnComponentBeginOverlap(RefillActivateZone)
  (params (OverlappedComponent :type Primitive%20Component%20Object%20Reference) (OtherActor :type Actor%20Object%20Reference) (OtherComp :type Primitive%20Component%20Object%20Reference) (OtherBodyIndex :type Integer) (bFromSweep :type Boolean) (SweepResult :type Hit%20Result%20Structure%20%28by%20ref%29))
  (bind _sm_bulletbox (Variables|Default|GetSM_BulletBox))
  (if (== OtherActor (Variables|Default|GetPlayerRef))
    (bind _outactors (Actor|GetAllActorsOfClass "/Game/Prototype_1/Weapons/Blueprints/BP_Pistol.BP_Pistol_C"))
    (bind _asbp_pistol (Utilities|Casting|CastToBP_Pistol (Utilities|Array|Get(acopy) _outactors)))
    (if (< (Variables|/Game/Prototype_1/Weapons/Blueprints/BP_WeaponBase.BP_WeaponBase_C|GetCurrentRemainingAmmo _asbp_pistol) 40)
      (Default|PickUpAmmo _asbp_pistol)
      (Audio|SpawnSoundatLocation "/Game/Prototype_1/Sounds/S_AmmoRefill.S_AmmoRefill" (Transformation|GetWorldLocation _sm_bulletbox) "0, 0, 0" 1.0 1.0 0.0 0 0)
      (Actor|DestroyActor (Components|GetOwner _sm_bulletbox)))))

(event EventBeginPlay
  (bind _outactors (Actor|GetAllActorsOfClass "/Game/Prototype_1/Core/Character/BP_PlayerCharacter.BP_PlayerCharacter_C"))
  (bind _asbp_player_character (Utilities|Casting|CastToBP_PlayerCharacter (Utilities|Array|Get(acopy) _outactors)))
  (Variables|Default|SetPlayerRef _asbp_player_character)
  (bind _uplocation (Timeline|Timeline_0 Play)
    (:Update
      (Transformation|AddRelativeLocation (Variables|Default|GetWidget_01) _uplocation false false)
      (Transformation|AddRelativeLocation (Variables|Default|GetWidget_02) _uplocation false false)
      (Transformation|AddRelativeLocation (Variables|Default|GetWidget_03) _uplocation false false))
    (:Finished
      (bind _downlocation (Timeline|Timeline_1 PlayFromStart)
        (:Update
          (Transformation|AddRelativeLocation (Variables|Default|GetWidget_01) _downlocation false false)
          (Transformation|AddRelativeLocation (Variables|Default|GetWidget_02) _downlocation false false)
          (Transformation|AddRelativeLocation (Variables|Default|GetWidget_03) _downlocation false false))
        (:Finished
          (Timeline|Timeline_0 PlayFromStart))))))

(event EventTick
  (params (DeltaSeconds :type Float%20%28single-precision%29))
  (Transformation|AddRelativeRotation (Variables|Default|GetWidget_01) (* (Math|Rotator|MakeRotator 0.0 0.0 1e+02) DeltaSeconds) false false))

(fn ConstructionScript)