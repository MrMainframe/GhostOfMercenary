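; BP_TeleportDoor is a door actor that teleports any actor entering its ActivateZone to a linked target door.
; On overlap it moves that actor to the location and rotation of the target's TeleportArrow component.
; Both doors clear their CanTeleport flag before the move and restore it after a short delay, so arrival does not immediately trigger a return trip.
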(event OnComponentBeginOverlap(ActivateZone)
  (params (OverlappedComponent :type Primitive%20Component%20Object%20Reference) (OtherActor :type Actor%20Object%20Reference) (OtherComp :type Primitive%20Component%20Object%20Reference) (OtherBodyIndex :type Integer) (bFromSweep :type Boolean) (SweepResult :type Hit%20Result%20Structure%20%28by%20ref%29))
  (bind _targetteleportdoor (Variables|Default|GetTargetTeleportDoor))
  (bind _output (Utilities|ResolveSoftReference _targetteleportdoor))
  (bind _teleportarrow (Variables|BP_TeleportDoor_C|GetTeleportArrow _output))
  (if (Variables|Default|GetbCanTeleport)
    (Variables|Default|SetbCanTeleport false)
    (Variables|BP_TeleportDoor_C|SetbCanTeleport _output false)
    (Transformation|Teleport OtherActor (Transformation|GetWorldLocation _teleportarrow) (Transformation|GetWorldRotation _teleportarrow))
    (Utilities|FlowControl|Delay 0.2)
    (Variables|BP_TeleportDoor_C|SetbCanTeleport (Utilities|ResolveSoftReference (Variables|Default|GetTargetTeleportDoor)) true)
    (Variables|Default|SetbCanTeleport true)))

(fn ConstructionScript)