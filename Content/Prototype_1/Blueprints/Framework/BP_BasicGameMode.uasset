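; Basic game mode that gates level completion on killing every enemy.
; On BeginPlay it counts all BP_AIBase actors, binds their post-death events to a kill counter, and hooks an event to the first BP_ToNextLevelDoor's next-level dispatcher.
; Its NextLevel event fires OnWin only when the kill count equals the enemy count taken at start.
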(event Custom|OnPostDead_Event
  (bind _result (Math|Integer|IncrementInt (Variables|Default|GetKillCount))
    (:%20%20
      (Variables|Default|SetKillCount _result))))

(event Custom|NextLevel
  (if (== (Variables|Default|GetEnemiesCount) (Variables|Default|GetKillCount))
    (Default|CallOnWin)))

(event EventBeginPlay
  (bind _outactors (Actor|GetAllActorsOfClass "/Game/Prototype_1/AI/BaseAI/System/AI/Blueprint/BP_AIBase.BP_AIBase_C"))
  (Variables|Default|SetEnemiesCount (Utilities|Array|Length _outactors))
  (for _array_element _outactors
    (Utilities|IsValid _array_element
      (:Is%20Valid
        (EventDispatchers|BindEventtoOnPostDead _array_element (delegate Custom|OnPostDead_Event)))))
  (bind _outactors_2 (Actor|GetAllActorsOfClass "/Game/Prototype_1/Blueprints/Actors/Doors/BP_ToNextLevelDoor.BP_ToNextLevelDoor_C"))
  (Utilities|IsValid (Utilities|Array|Get(acopy) _outactors_2)
    (:Is%20Valid
      (EventDispatchers|BindEventtoToNextLevel (Utilities|Array|Get(acopy) _outactors_2) (EventDispatchers|CreateEvent :!event Custom|NextLevel)))))

(fn ConstructionScript)